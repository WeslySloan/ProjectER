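; BP_TEMP_HUD is a temporary HUD Blueprint that shows the screen widget for the current level.
; On BeginPlay it compares the current level name against the main menu and lobby level names.
; It creates the matching main menu or lobby HUD widget, falling back to the OutGame widget for any other level, and adds it to the viewport.
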(event EventBeginPlay
  (bind _returnvalue (Game|GetCurrentLevelName true))
  (bind _output_get (Variables|Default|SetCurrentLevelName (Utilities|String|StringToName _returnvalue)))
  (if (== _output_get (Variables|Default|GetMainMenuLevelName))
    (bind _returnvalue_2 (UserInterface|CreateWidget "/Game/JMS/TEMP_Widget/WBP_TEMP_MainMenuHUD.WBP_TEMP_MainMenuHUD_C"))
    (UserInterface|Viewport|AddtoViewport _returnvalue_2 0)
    (elif (== (Variables|Default|GetCurrentLevelName) (Variables|Default|GetLobbyLevelName))
      (bind _returnvalue_3 (UserInterface|CreateWidget "/Game/JMS/TEMP_Widget/WBP_TEMP_LobbyHUD.WBP_TEMP_LobbyHUD_C"))
      (UserInterface|Viewport|AddtoViewport _returnvalue_3 0)
      (else
        (bind _returnvalue_4 (UserInterface|CreateWidget "/Game/JMS/TEMP_Widget/WBP_TEMP_OutGame.WBP_TEMP_OutGame_C"))
        (UserInterface|Viewport|AddtoViewport _returnvalue_4 0)))))

(event Collision|EventActorBeginOverlap
  (params (OtherActor :type Actor%20Object%20Reference)))

(event EventTick
  (params (DeltaSeconds :type Float%20%28single-precision%29)))

(fn ConstructionScript)