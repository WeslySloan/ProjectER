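; Gameplay ability for a monster's auto attack against its target player.
; On activation it resets attack utility, then ends if the monster's own health is depleted, clearing the target.
; Otherwise it faces the target, starts an attack-speed-based cooldown and plays the attack montage from monster data.
; The montage's hit gameplay event applies the damage effect to the target, and montage end or interruption ends the ability.
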(event Ability|EventActivateAbility
  (Ability|CommitAbility)
  (bind _asbase_monster (Utilities|Casting|CastToBaseMonster (Ability|GetOwningActorfromActorInfo)))
  ;[0.15 0.15 0.15 0.5] Target Look
  (Variables|/Script/ProjectER.BaseMonster|SetAttackUtility _asbase_monster 0.0)
  ;[0.15 0.15 0.15 0.5] Target Die Check
  (if (<= (.currentvalue (Variables|/Script/ProjectER.BaseAttributeSet|GetHealth (Variables|/Script/ProjectER.BaseMonster|GetAttributeSet _asbase_monster))) 0.0)
    (Variables|/Script/ProjectER.BaseMonster|SetTargetPlayer _asbase_monster 0)
    (Ability|EndAbility)
    (else
      (Transformation|SetActorRotation _asbase_monster (Math|Rotator|FindLookatRotation (Transformation|GetActorLocation _asbase_monster) (Transformation|GetActorLocation (Variables|/Script/ProjectER.BaseMonster|GetTargetPlayer _asbase_monster))))
      (Class|BaseMonster|OnCooldown _asbase_monster "(TagName=\"Cooldown.AutoAttack\")" (.currentvalue (Variables|/Script/ProjectER.BaseAttributeSet|GetAttackSpeed (Variables|/Script/ProjectER.BaseMonster|GetAttributeSet _asbase_monster))))
      ;[0.15 0.15 0.15 0.5] Damage
      (|PlayMontageandWaitProxy "None" (.Value (Utilities|Map|Find (Variables|/Script/ProjectER.MonsterDataAsset|GetMontages (Variables|/Script/ProjectER.BaseMonster|GetMonsterData _asbase_monster)) "Attack")) 1.0 "None" true 1.0 0.0 false
        (:then
          (Ability|Tasks|WaitGameplayEvent "(TagName=\"Event.Montage.AttackHit\")" 0
            (:EventReceived
              (GameplayEffects|ApplyGameplayEffectToTarget :self (Ability|GetAbilitySystemComponent _asbase_monster) :GameplayEffectClass "/Game/BCW/GAS/GE/GE_MonsterAttackDamage.GE_MonsterAttackDamage_C" :Target (Ability|GetAbilitySystemComponent (Variables|/Script/ProjectER.BaseMonster|GetTargetPlayer _asbase_monster))))))
        (:OnCompleted
          (Ability|EndAbility :!label _label))
        (:OnBlendOut
          (goto _label))
        (:OnInterrupted
          (goto _label))
        (:OnCancelled
          (goto _label))))))