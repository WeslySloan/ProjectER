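; Gameplay ability that makes a monster chase its target player until within attack range.
; On activation it applies GE_MonsterChase, flags the monster as in combat and runs AIMoveTo, with acceptance radius set to the AttackRange attribute minus the target's capsule radius.
; The ability ends when the move succeeds or fails; on end it removes the effect and calls SendAttackRangeEvent with the attack range.
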(event Ability|EventActivateAbility
  (bind _returnvalue (Ability|GetOwningActorfromActorInfo))
  (bind _returnvalue_2 (Ability|GetAbilitySystemComponent _returnvalue))
  (Ability|CommitAbility)
  (bind _returnvalue_3 (GameplayEffects|ApplyGameplayEffectToSelf :self _returnvalue_2 :GameplayEffectClass "/Game/BCW/GAS/GE/StateTreeGE/GE_MonsterChase.GE_MonsterChase_C"))
  (bind _returnvalue_4 (GameplayAttributes|GetAttributeSet _returnvalue_2 "/Script/ProjectER.BaseMonsterAttributeSet"))
  (bind _asbase_monster (Utilities|Casting|CastToBaseMonster _returnvalue))
  (Variables|/Script/ProjectER.BaseMonster|SetbIsCombat _asbase_monster true)
  (bind _ascharacter (Utilities|Casting|CastToCharacter (Variables|/Script/ProjectER.BaseMonster|GetTargetPlayer _asbase_monster)))
  (AI|AIMoveTo _asbase_monster "0, 0, 0" _ascharacter (- (.currentvalue (Variables|/Script/ProjectER.BaseAttributeSet|GetAttackRange _returnvalue_4)) (Components|Capsule|GetScaledCapsuleRadius (Variables|/Script/Engine.Character|GetCapsuleComponent _ascharacter))) false
    (:OnSuccess
      _)
    (:OnFail
      _))
  (Ability|EndAbility))

(event Ability|EventOnEndAbility
  (params (bWasCancelled :type Boolean))
  (GameplayEffects|RemoveActiveGameplayEffect (Ability|GetAbilitySystemComponent (Ability|GetOwningActorfromActorInfo)) (stale Ability|EventActivateAbility _returnvalue_3) -1)
  (Class|BaseMonster|SendAttackRangeEvent (stale Ability|EventActivateAbility _asbase_monster) (.currentvalue (Variables|/Script/ProjectER.BaseAttributeSet|GetAttackRange (stale Ability|EventActivateAbility _returnvalue_4)))))