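; Boss gameplay ability that plays a monster's FlyEnd montage to end its flying state.
; On activation it commits, applies GE_MonsterFlyEnd to itself to drive a gameplay cue, and plays the montage looked up from the monster's data.
; The ability ends when the montage completes, blends out, is interrupted or cancelled, and OnEndAbility removes the effect.
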(event Ability|EventActivateAbility
  (bind _returnvalue (Ability|GetOwningActorfromActorInfo))
  (Ability|CommitAbility)
  (bind _asbase_monster (Utilities|Casting|CastToBaseMonster _returnvalue))
  ;[0.15 0.15 0.15 0.5] Cue 실행용 GE
  (bind _returnvalue_2 (GameplayEffects|ApplyGameplayEffectToSelf :self (Ability|GetAbilitySystemComponent _returnvalue) :GameplayEffectClass "/Game/BCW/GAS/GE/StateTreeGE/Boss/GE_MonsterFlyEnd.GE_MonsterFlyEnd_C"))
  (|PlayMontageandWaitProxy "None" (.Value (Utilities|Map|Find (Variables|/Script/ProjectER.MonsterDataAsset|GetMontages (Variables|/Script/ProjectER.BaseMonster|GetMonsterData _asbase_monster)) "FlyEnd")) 1.0 "None" true 1.0 0.0 false
    (:OnCompleted
      _)
    (:OnBlendOut
      _)
    (:OnInterrupted
      _)
    (:OnCancelled
      _))
  (Ability|EndAbility))

(event Ability|EventOnEndAbility
  (params (bWasCancelled :type Boolean))
  (GameplayEffects|RemoveActiveGameplayEffect (Ability|GetAbilitySystemComponent (Ability|GetOwningActorfromActorInfo)) (stale Ability|EventActivateAbility _returnvalue_2) -1))