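; GA_TryRevive is a gameplay ability that lets a character revive a downed teammate nearby.
; After committing, it sphere-overlaps pawns around the avatar and takes the first same-team BaseCharacter tagged State.Life.Down, ending if none is found.
; It plays the revive montage alongside a ReviveTime delay, after which the authority calls Revive on the target and ends the ability.
; Montage interruption or cancellation ends the ability early.
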(event Ability|EventActivateAbility
  (bind _returnvalue (Ability|GetAvatarActorfromActorInfo))
  ;[0.15 0.15 0.15 0.5] Start & Initialize
  (bind _asbase_character (Utilities|Casting|CastToBaseCharacter (Ability|GetAvatarActorfromActorInfo)))
  (Variables|Default|SetOwner%20Actor _asbase_character)
  (Variables|Default|SetOwner%20ASC (Ability|GetAbilitySystemComponent _asbase_character))
  (bind _returnvalue_2 (Ability|CommitAbility))
  (if _returnvalue_2
    (Utilities|FlowControl|Sequence
      (:then_0
        ;[0.15 0.15 0.15 0.5] Sphere Overlap
        (bind _outactors (Collision|SphereOverlapActors (Transformation|GetActorLocation _returnvalue) (Variables|Default|GetRevive%20Radius) (Utilities|Array|MakeArray "ObjectTypeQuery3") 0 (Utilities|Array|MakeArray _returnvalue)))
        (bind _array_element (Utilities|Array|ForEachLoopwithBreak _outactors :!label _label)
          (:LoopBody
            (bind _asbase_character_2 (Utilities|Casting|CastToBaseCharacter _array_element))
            (if (and (Utilities|Enum|Equal(Enum) (Variables|/Script/ProjectER.BaseCharacter|GetTeamID _asbase_character_2) (Variables|/Script/ProjectER.BaseCharacter|GetTeamID (Variables|Default|GetOwner%20Actor))) (GameplayTags|HasMatchingGameplayTag (Ability|GetAbilitySystemComponent _asbase_character_2) "(TagName=\"State.Life.Down\")"))
              (Variables|Default|SetTarget%20Actor _asbase_character_2)
              (goto _label Break)))
          (:Completed
            ;[0.15 0.15 0.15 0.5] Play Montage and Revive
            (Utilities|IsValid (Variables|Default|GetTarget%20Actor)
              (:Is%20Valid
                (Utilities|FlowControl|Sequence
                  (:then_0
                    (Ability|Tasks|WaitDelay (Variables|Default|GetRevive%20Time)
                      (:OnFinish
                        (Ability|HasAuthority
                          (:True
                            (Class|BaseCharacter|Revive (Variables|Default|GetTarget%20Actor) (Transformation|GetActorLocation (Variables|Default|GetTarget%20Actor)))
                            (Ability|EndAbility))))))
                  (:then_1
                    (|PlayMontageandWaitProxy "None" "/Game/KTW/Character/Animation/AM_Revive.AM_Revive" 1.0 "None" true 1.0 0.0 false
                      (:OnInterrupted
                        _)
                      (:OnCancelled
                        _))
                    (Ability|EndAbility))))
              (:Is%20Not%20Valid
                (Ability|EndAbility)))))))
    (else
      (Ability|EndAbility))))

(event Ability|EventOnEndAbility
  (params (bWasCancelled :type Boolean)))