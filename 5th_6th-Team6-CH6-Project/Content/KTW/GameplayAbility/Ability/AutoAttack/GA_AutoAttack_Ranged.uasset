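; Gameplay ability for a hero's ranged auto attack, firing a homing projectile at the target cached on activation.
; After commit, it plays the attack montage at a rate read from an ASC attribute and ends when the montage finishes or is interrupted.
; A montage gameplay event makes the server spawn the HeroData projectile class from the muzzle along the combat gaze, passing it a SetByCaller damage effect spec to apply.
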(event Ability|EventActivateAbility
  ;[0.15 0.15 0.15 0.5] Start & Initialize
  (bind _asbase_character (Utilities|Casting|CastToBaseCharacter (Ability|GetAvatarActorfromActorInfo)))
  (Variables|Default|SetOwnerActor _asbase_character)
  (Variables|Default|SetOwnerASC (Ability|GetAbilitySystemComponent _asbase_character))
  (Variables|Default|SetCached%20Target%20Actor (Variables|/Script/ProjectER.BaseCharacter|GetTargetActor _asbase_character))
  (bind _returnvalue (Ability|CommitAbility))
  (if _returnvalue
    (Utilities|FlowControl|Sequence
      (:then_0
        ;[0.15 0.15 0.15 0.5] Wait Event & Spawn Actor
        (Ability|Tasks|WaitGameplayEvent "(TagName=\"Event.Montage.SpawnProjectile\")" 0 true
          (:then
            (bind _returnvalue_2 (Class|BaseCharacter|GetMuzzleLocation (Variables|Default|GetOwnerActor) (Variables|/Script/ProjectER.CharacterData|GetMuzzleSocketName (Variables|/Script/ProjectER.BaseCharacter|GetHeroData (Variables|Default|GetOwnerActor)))))
            (bind _returnvalue_3 (Class|BaseCharacter|GetCombatGazeRotation (Variables|Default|GetOwnerActor) (Variables|/Script/ProjectER.CharacterData|GetMuzzleSocketName (Variables|/Script/ProjectER.BaseCharacter|GetHeroData (Variables|Default|GetOwnerActor)))))
            (bind _returnvalue_4 (Ability|GameplayEffect|AssignTagSetbyCallerMagnitude (GameplayEffects|MakeOutgoingSpec (Variables|Default|GetOwnerASC) "/Game/KTW/GameplayAbility/Effect/GE_AutoAttack_Damage.GE_AutoAttack_Damage_C" 1.0 (GameplayEffects|MakeEffectContext (Variables|Default|GetOwnerASC))) "(TagName=\"Data.Amount.Damage\")" 1e+01)))
          (:EventReceived
            (Ability|HasAuthority
              (:True
                (Game|SpawnActorfromClass (Variables|/Script/ProjectER.CharacterData|GetProjectileClass (Variables|/Script/ProjectER.BaseCharacter|GetHeroData (Variables|Default|GetOwnerActor))) (Math|Transform|MakeTransform _returnvalue_2 _returnvalue_3 "1.000000,1.000000,1.000000") "AlwaysSpawn" "MultiplyWithRoot" 0 "/Game/KTW/Character/Data/DA_ProjectileData.DA_ProjectileData" _returnvalue_4 (Variables|Default|GetCached%20Target%20Actor) (Variables|Default|GetOwnerActor)))))))
      (:then_1
        ;[0.15 0.15 0.15 0.5] Play Montage
        (|PlayMontageandWaitProxy "None" "/Game/KTW/Character/Animation/AM_BaseCharacter_AutoAttack_Ranged.AM_BaseCharacter_AutoAttack_Ranged" (.ReturnValue (Ability|Attribute|GetFloatAttributefromAbilitySystemComponent (Variables|Default|GetOwnerASC) "(AttributeName=\"AttackSpeed\",Attribute=/Script/ProjectER.BaseAttributeSet:AttackSpeed,AttributeOwner=\"/Script/CoreUObject.Class'/Script/ProjectER.BaseAttributeSet'\")")) "None" true 1.0 0.0 false
          (:OnCompleted
            _)
          (:OnInterrupted
            _)
          (:OnCancelled
            _))
        (Ability|EndAbility)))
    (else
      (Ability|EndAbility))))