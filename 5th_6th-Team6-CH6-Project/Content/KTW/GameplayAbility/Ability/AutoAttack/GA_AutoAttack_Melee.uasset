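; Gameplay ability for a character's melee auto attack, damaging the target cached from the avatar at activation.
; After commit, it plays the attack montage at a rate read from an attribute while waiting for the AttackHit gameplay event.
; The event applies a damage effect with a fixed SetByCaller magnitude to that target, then ends the ability.
; Montage completion, blend-out, interruption, cancellation or a failed commit also ends it.
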(event Ability|EventActivateAbility
  ;[0.15 0.15 0.15 0.5] Start & Initialize
  (bind _asbase_character (Utilities|Casting|CastToBaseCharacter (Ability|GetAvatarActorfromActorInfo)))
  (Variables|Default|SetCached%20Target%20Actor (Variables|/Script/ProjectER.BaseCharacter|GetTargetActor _asbase_character))
  (bind _returnvalue (Ability|CommitAbility))
  (if _returnvalue
    (Utilities|FlowControl|Sequence
      (:then_0
        (Ability|Tasks|WaitGameplayEvent "(TagName=\"Event.Montage.AttackHit\")" 0
          (:EventReceived
            (bind _returnvalue_2 (Ability|GameplayEffect|AssignTagSetbyCallerMagnitude (GameplayEffects|MakeOutgoingSpec (Ability|GetAbilitySystemComponent _asbase_character) "/Game/KTW/GameplayAbility/Effect/GE_AutoAttack_Damage.GE_AutoAttack_Damage_C" 1.0 (GameplayEffects|MakeEffectContext (Ability|GetAbilitySystemComponent _asbase_character))) "(TagName=\"Data.Amount.Damage\")" 1e+01))
            (GameplayEffects|ApplyGameplayEffectSpecToTarget _returnvalue_2 (Ability|TargetData|AbilityTargetDatafromActor (Variables|Default|GetCached%20Target%20Actor)))
            (Ability|EndAbility))))
      (:then_1
        ;[0.15 0.15 0.15 0.5] Play Montage
        (|PlayMontageandWaitProxy "None" "/Game/KTW/Character/Animation/AM_BaseCharacter_AutoAttack_Melee.AM_BaseCharacter_AutoAttack_Melee" (.ReturnValue (Ability|Attribute|GetFloatAttributefromAbilitySystemComponent (Ability|GetAbilitySystemComponent _asbase_character) "(AttributeName=\"AttackSpeed\",Attribute=/Script/ProjectER.BaseAttributeSet:AttackSpeed,AttributeOwner=\"/Script/CoreUObject.Class'/Script/ProjectER.BaseAttributeSet'\")")) "None" true 1.0 0.0 false
          (:OnCompleted
            _)
          (:OnBlendOut
            _)
          (:OnInterrupted
            _)
          (:OnCancelled
            _))
        (Ability|EndAbility)))
    (else
      (Ability|EndAbility))))

(event Ability|EventOnEndAbility
  (params (bWasCancelled :type Boolean)))