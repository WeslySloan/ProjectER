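; BP_BaseCharacter is a base character Blueprint that acts as a line-of-sight vision provider.
; On BeginPlay it registers its LineOfSight component with the LOS Vision Subsystem on that component's vision channel.
; Tick, the custom tick event and the construction script are empty.
; Disconnected leftover nodes hold a Curved World camera update with debug printing, a looping timer and an UpdateCameraLOS call, none of which run.
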(event Custom|custom%20tick)

(event EventBeginPlay
  (bind _lineofsight (Variables|Default|GetLineOfSight))
  (Utilities|FlowControl|Sequence
    (:then_2
      ;[0.15 0.15 0.15 0.5] Register to Vision Subsystem
      (Class|LOSVisionSubsystem|RegisterProvider (Subsystems|GetLOSVisionSubsystem) _lineofsight (Class|LineOfSightComponent|GetVisionChannel _lineofsight)))))

(event EventTick
  (params (DeltaSeconds :type Float%20%28single-precision%29)))

(fn ConstructionScript)