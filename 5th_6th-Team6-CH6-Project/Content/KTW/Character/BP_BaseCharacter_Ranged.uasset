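; BP_BaseCharacter_Ranged is a ranged character base Blueprint that supplies line-of-sight vision through its LineOfSight component.
; On BeginPlay it registers that component with the WorldObstacleSubsystem as a provider on the component's vision channel.
; Tick updates the local LOS stamp every frame.
; BeginPlay also starts a looping timer at roughly 60 Hz, and the custom tick event in the graph is empty.
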(event Custom|custom%20tick)

(event EventBeginPlay
  (bind _lineofsight (Variables|Default|GetLineOfSight))
  (Utilities|FlowControl|Sequence
    (:then_1
      ;[0.15 0.15 0.15 0.5] Register to Vision Subsystem
      (Class|WorldObstacleSubsystem|RegisterProvider (Subsystems|GetWorldObstacleSubsystem) _lineofsight (Class|LineOfSightComponent|GetVisionChannel _lineofsight)))
    (:then_2
      (Utilities|Time|SetTimerbyEvent (EventDispatchers|CreateEvent :!event Custom|custom%20tick) 0.016667 true))))

(event EventTick
  (params (DeltaSeconds :type Float%20%28single-precision%29))
  (Utilities|FlowControl|Sequence
    (:then_1
      ;[0.15 0.15 0.15 0.5] update local LOS Stamp
      (Class|LineOfSightComponent|UpdateLocalLOS (Variables|Default|GetLineOfSight)))))

(fn ConstructionScript)