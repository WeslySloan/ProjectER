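; BP_WorldBaker is a world baker actor that can show its last baked obstacle texture on a debug plane.
; The construction script rotates the plane with BoxVolume and sizes it as a square from the box's X extent and scale only.
; On BeginPlay, ShowDebugPlane either applies a dynamic visualizer material fed with LastBakedTexture or hides the plane in game.
; The baking itself is not done in these graphs.
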(event EventBeginPlay
  (if (Variables|Default|GetbShowDebugPlane)
    (bind _returnvalue (Rendering|Material|CreateDynamicMaterialInstance "/Game/PSM/WorldBaker/M_WorldObstacleVisualizer.M_WorldObstacleVisualizer" "None" "Transient" :!class /Script/Engine.KismetMaterialLibrary))
    (Rendering|Material|SetTextureParameterValue _returnvalue "WorldObstacleTexture" (Variables|Default|GetLastBakedTexture))
    (Rendering|Material|SetMaterial (Variables|Default|GetDebugVisualizer) 0 _returnvalue)
    (else
      (Development|SetHiddeninGame (Variables|Default|GetDebugVisualizer) true false))))

(event Collision|EventActorBeginOverlap
  (params (OtherActor :type Actor%20Object%20Reference)))

(event EventTick
  (params (DeltaSeconds :type Float%20%28single-precision%29)))

(fn ConstructionScript
  (bind _debugvisualizer (Variables|Default|GetDebugVisualizer))
  (bind _boxvolume (Variables|Default|GetBoxVolume))
  (bind _returnvalue (Transformation|GetWorldScale _boxvolume))
  (bind _boxextent (Variables|/Script/Engine.BoxComponent|GetBoxExtent _boxvolume))
  (bind _returnvalue_2 (/ (.x _boxextent) 1e+02))
  (bind _returnvalue_3 (* _returnvalue_2 2.0))
  (bind _returnvalue_4 (* (.x _returnvalue) _returnvalue_3))
  (Transformation|SetWorldScale3D _debugvisualizer (Math|Vector|MakeVector _returnvalue_4 _returnvalue_4 1.0))
  (Transformation|SetWorldRotation _debugvisualizer (Transformation|GetWorldRotation (Variables|Default|GetBoxVolume)) false false))