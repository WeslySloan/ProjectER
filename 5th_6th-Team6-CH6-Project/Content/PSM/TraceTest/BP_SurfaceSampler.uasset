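; BP_SurfaceSampler is a test actor for baking and visualizing surface sample points through a VisibilityTargetComp.
; On BeginPlay it sets the Box component as the target shape and bakes the sample points, then debug-draws them every Tick.
; Sphere and Capsule references, construction-time baking and an IsFullyHiddenByVolumes visibility printout remain as disconnected nodes that never run.
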(event EventBeginPlay
  (Class|VisibilityTargetComp|SetTargetShapeComp (Variables|Default|GetVisibilityTargetComp) (Variables|Default|GetBox))
  (Class|VisibilityTargetComp|BakeSamplePoints (Variables|Default|GetVisibilityTargetComp)))

(event Collision|EventActorBeginOverlap
  (params (OtherActor :type Actor%20Object%20Reference)))

(event EventTick
  (params (DeltaSeconds :type Float%20%28single-precision%29))
  (Class|VisibilityTargetComp|DebugDrawSamplePoints (Variables|Default|GetVisibilityTargetComp) 0.0))

(fn ConstructionScript)