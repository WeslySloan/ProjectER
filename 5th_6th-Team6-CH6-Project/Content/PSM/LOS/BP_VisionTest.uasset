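; BP_VisionTest is a test actor for the line-of-sight vision system.
; On BeginPlay it registers its LineOfSight component with the LOS vision subsystem under that component's vision channel and prints the result.
; An optional debug plane, scaled to the vision range, shows the component's LOS material.
; A looping timer of about 30 Hz is started, but TracingUpdateTick is empty and the detection and height-texture test nodes are disconnected.
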(event Custom|TracingUpdateTick)

(event EventBeginPlay
  (bind _debugplane (Variables|Default|GetDebugPlane))
  (bind _lineofsight (Variables|Default|GetLineOfSight))
  (bind _lineofsight_2 (Variables|Default|GetLineOfSight))
  (bind _lineofsight_3 (Variables|Default|GetLineOfSight))
  (bind _returnvalue (Class|LineOfSightComponent|GetLOSMaterialMID _lineofsight_3))
  (bind _returnvalue_2 (Class|LineOfSightComponent|GetVisionChannel _lineofsight))
  (bind _visionrange (Variables|/Script/TopDownVision.LineOfSightComponent|GetVisionRange _lineofsight_2))
  (bind _returnvalue_3 (/ _visionrange 1e+02))
  (bind _returnvalue_4 (* _returnvalue_3 2.0))
  (Utilities|FlowControl|Sequence
    (:then_0
      ;[0.15 0.15 0.15 0.5] Register LOS to the SubSystem
      (bind _returnvalue_5 (Class|LOSVisionSubsystem|RegisterProvider (Subsystems|GetLOSVisionSubsystem) _lineofsight _returnvalue_2))
      (Development|PrintString (Utilities|String|ToString(Text) (Utilities|Text|FormatText "Register {did worked?} Name:{name}" (Utilities|String|SelectText "Successful" "failed" _returnvalue_5) (Utilities|Name|EnumtoName _returnvalue_2))) true false)
      (if (Variables|Default|GetbShowDebugPlane)
        ;[0.15 0.15 0.15 0.5] Draw LOD stamp to the plane for debug
        (Utilities|IsValid _returnvalue
          (:Is%20Valid
            (Rendering|Material|SetMaterial _debugplane 0 _returnvalue)
            (Transformation|SetRelativeScale3D _debugplane (Math|Vector|MakeVector _returnvalue_4 _returnvalue_4 _returnvalue_4)))
          (:Is%20Not%20Valid
            (Development|PrintString "Invalid MID" true true "(R=1.000000,G=0.000000,B=0.014383,A=1.000000)")))
        (else
          (Rendering|SetVisibility (Variables|Default|GetDebugPlane) false false))))
    (:then_2
      (Utilities|Time|SetTimerbyEvent (EventDispatchers|CreateEvent :!event Custom|TracingUpdateTick) 0.033333 true))))

(event Collision|EventActorBeginOverlap
  (params (OtherActor :type Actor%20Object%20Reference)))

(fn ConstructionScript)

(fn InitializeLOS)